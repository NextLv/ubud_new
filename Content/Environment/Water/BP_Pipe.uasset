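; BP_Pipe is a water environment actor that builds a pipe along an editable spline.
; The construction script loops over the spline points, adding a spline mesh component with the chosen static mesh on each pass.
; Each mesh takes local positions and tangents from the current index and two indices earlier, rather than from adjacent points.
; It has no active runtime logic.
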(event EventBeginPlay)

(event Collision|EventActorBeginOverlap
  (params (OtherActor :type Actor%20Object%20Reference)))

(event EventTick
  (params (DeltaSeconds :type Float%20%28single-precision%29)))

(fn ConstructionScript
  (bind _spline (Variables|Default|GetSpline))
  (bind _output_get (Variables|Default|SetNumber%20of%20Spline (Spline|GetNumberOfSplinePoints (Variables|Default|GetSpline))))
  (for _index (range 1 (- _output_get 1))
    (bind _returnvalue (AddComponent|AddSplineMeshComponent false))
    (SplineMesh|SetStartandEnd _returnvalue (.Location (Spline|GetLocationandTangentatSplinePoint _spline (- _index 2) "Local")) (.Tangent (Spline|GetLocationandTangentatSplinePoint _spline (- _index 2) "Local")) (.Location (Spline|GetLocationandTangentatSplinePoint _spline _index "Local")) (.Tangent (Spline|GetLocationandTangentatSplinePoint _spline _index "Local")) true :!class /Script/Engine.SplineMeshComponent)
    (Components|StaticMesh|SetStaticMesh _returnvalue (Variables|Default|GetStaticMesh))))